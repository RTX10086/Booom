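; BP_Function holds a Find Target helper that looks for a third-person character or BP_NEnemy between a player character and its MouseLocation.
; It box-traces WorldDynamic objects from the actor's location, with persistent debug drawing, and casts the hit actor to either type.
; A match returns Find true with both typed targets.
; The Find false return and a forward-vector end point are left unconnected.
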(fn FindTarget
  (params (NewParam :type Actor%20Object%20Reference))
  (bind _asbp_third_person_character (Utilities|Casting|CastToBP_ThirdPersonCharacter NewParam))
  (LocalVariables|SetEndLocation (Variables|/Game/ThirdPerson/Blueprints/BP_ThirdPersonCharacter.BP_ThirdPersonCharacter_C|GetMouseLocation _asbp_third_person_character))
  (bind (_outhit _returnvalue) (Class|KismetSystemLibrary|BoxTraceSingleforObjects 0 (Transformation|GetActorLocation NewParam) (LocalVariables|GetEndLocation) "0.000000,50.000000,90.000000" "0.000000,0.000000,0.000000" (Utilities|Array|MakeArray (Utilities|Enum|LiteralenumEObjectTypeQuery "ObjectTypeQuery2")) false 0 "Persistent" true))
  (if _returnvalue
    (bind _asbp_third_person_character_2 (Utilities|Casting|CastToBP_ThirdPersonCharacter (.HitActor (Collision|BreakHitResult _outhit)))
      (:then
        _)
      (:CastFailed
        (bind _asbp_nenemy (Utilities|Casting|CastToBP_NEnemy (.HitActor (Collision|BreakHitResult _outhit)) :!label _label))))
    (else
      (goto _label)))
  (return true _asbp_third_person_character_2 _asbp_nenemy))