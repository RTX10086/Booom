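; BP_Weapon_Gun is a gun weapon that fires bullet actors when attacked with and flags the third-person character as armed on touch.
; The attack event calls the parent, then, if ready, messages the player to play the attack animation and spawns BulletClass at the muzzle (发射口), passing itself to the bullet.
; A one-shot timer using the attack rate from Info re-enables firing.
; Overlapping its Sphere sets the character's HaveAGun flag.
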(event OnComponentBeginOverlap(Sphere)
  (params (OverlappedComponent :type Primitive%20Component%20Object%20Reference) (OtherActor :type Actor%20Object%20Reference) (OtherComp :type Primitive%20Component%20Object%20Reference) (OtherBodyIndex :type Integer) (bFromSweep :type Boolean) (SweepResult :type Hit%20Result%20Structure%20%28by%20ref%29))
  (bind _asbp_third_person_character (Utilities|Casting|CastToBP_ThirdPersonCharacter OtherActor))
  (Variables|/Game/ThirdPerson/Blueprints/BP_ThirdPersonCharacter.BP_ThirdPersonCharacter_C|SetHave%20a%20Gun? _asbp_third_person_character true))

(event Custom|发射子弹
  (if (Variables|Default|Get是否可以攻击)
    (Class|BPIPlayer|攻击动画(Message) (Game|GetPlayerCharacter 0))
    (bind _returnvalue (Game|SpawnActorfromClass (Variables|Default|GetBulletClass) (Transformation|GetWorldTransform (Variables|Default|Get发射口)) "Undefined" 0 0))
    (bind _asbp_bullets (Utilities|Casting|CastToBP_Bullets _returnvalue))
    (Variables|/Game/BP/Weapon/BP_Bullets.BP_Bullets_C|SetGun _asbp_bullets self)
    (Variables|Default|Set是否可以攻击 false)
    (Utilities|Time|SetTimerbyEvent (delegate Custom|定时器) (Utilities|Struct|BreakS_WeaponInfo (Variables|Default|GetInfo)))))

(event Custom|定时器
  (Variables|Default|Set是否可以攻击 true))

(event EventBeginPlay
  (|CallParentFunction) ; 此节点被禁用，将不会被调用。\n从引脚连出引线来编译功能。
)

(event Collision|EventActorBeginOverlap
  (params (OtherActor :type Actor%20Object%20Reference))
  (|CallParentFunction OtherActor) ; 此节点被禁用，将不会被调用。\n从引脚连出引线来编译功能。
)

(event Event武器攻击
  (|CallParentFunction)
  (CallFunction|发射子弹))

(fn ConstructionScript
  (|CallParentFunction))