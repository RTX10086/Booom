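; BP_Weapon is a weapon actor the third-person character can pick up, with a widget that shows its attributes.
; On BeginPlay it hides the widget and passes itself to UMG_PickUpWeapon for the attribute display.
; Sphere overlap shows or hides the widget and reports pickup range to BP_ThirdPersonCharacter through the 拾取武器 (pick up weapon) message.
; The 武器攻击 (weapon attack) event is an empty stub.
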(event OnComponentBeginOverlap(Sphere)
  (params (OverlappedComponent :type Primitive%20Component%20Object%20Reference) (OtherActor :type Actor%20Object%20Reference) (OtherComp :type Primitive%20Component%20Object%20Reference) (OtherBodyIndex :type Integer) (bFromSweep :type Boolean) (SweepResult :type Hit%20Result%20Structure%20%28by%20ref%29))
  (bind _asbp_third_person_character (Utilities|Casting|CastToBP_ThirdPersonCharacter OtherActor))
  (Class|BPIPlayer|拾取武器(Message) _asbp_third_person_character self true)
  (Rendering|SetVisibility (Variables|Default|GetWidget) true false))

(event OnComponentEndOverlap(Sphere)
  (params (OverlappedComponent :type Primitive%20Component%20Object%20Reference) (OtherActor :type Actor%20Object%20Reference) (OtherComp :type Primitive%20Component%20Object%20Reference) (OtherBodyIndex :type Integer))
  (bind _asbp_third_person_character (Utilities|Casting|CastToBP_ThirdPersonCharacter OtherActor))
  (Class|BPIPlayer|拾取武器(Message) _asbp_third_person_character 0 false)
  (Rendering|SetVisibility (Variables|Default|GetWidget) false false))

(event Custom|武器攻击)

(event EventBeginPlay
  (bind _widget (Variables|Default|GetWidget))
  (bind _asumg_pick_up_weapon (Utilities|Casting|CastToUMG_PickUpWeapon (UserInterface|GetWidget _widget)))
  (Rendering|SetVisibility _widget false false)
  (bind _output_get (Variables|Default|SetAs%20UMG%20Pick%20Up%20Weapon _asumg_pick_up_weapon))
  (Default|武器属性显示 _output_get self))

(fn ConstructionScript)