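; BP_子弹盒 is an ammo box pickup that refills the player's gun when the character overlaps its sphere.
; It checks that the BP_ThirdPersonCharacter's current weapon is a gun whose bullet type (子弹种类) matches the box's NewVar, then calls UpdateBulletAmount with a fixed amount and destroys itself.
; Otherwise, it briefly shows a "无法拾取" (cannot pick up) prompt on the character's main UMG widget and hides it after a delay.
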(event OnComponentBeginOverlap(Sphere)
  (params (OverlappedComponent :type Primitive%20Component%20Object%20Reference) (OtherActor :type Actor%20Object%20Reference) (OtherComp :type Primitive%20Component%20Object%20Reference) (OtherBodyIndex :type Integer) (bFromSweep :type Boolean) (SweepResult :type Hit%20Result%20Structure%20%28by%20ref%29))
  (bind _asbp_third_person_character (Utilities|Casting|CastToBP_ThirdPersonCharacter OtherActor))
  (Variables|Default|SetAs%20BP%20Third%20Person%20Character _asbp_third_person_character)
  (bind _asbp_weapon_gun (Utilities|Casting|CastToBP_Weapon_Gun (Variables|/Game/ThirdPerson/Blueprints/BP_ThirdPersonCharacter.BP_ThirdPersonCharacter_C|GetCurrentWeapon _asbp_third_person_character))
    (:then
      (if (== (Utilities|Struct|BreakS_GunAttribute (Variables|/Game/BP/Weapon/BP_Weapon_Gun.BP_Weapon_Gun_C|GetGunInfo _asbp_weapon_gun)) (Variables|Default|GetNewVar))
        (Default|UpdateBulletAmount _asbp_weapon_gun 20)
        (Actor|DestroyActor)
        (else
          (Widget|SetVisibility (Variables|/Game/UI/UMG/UMG_Main.UMG_Main_C|GetTextBlock_提示 (Variables|/Game/ThirdPerson/Blueprints/BP_ThirdPersonCharacter.BP_ThirdPersonCharacter_C|GetUMG_Main (Variables|Default|GetAs%20BP%20Third%20Person%20Character))) "HitTestInvisible" :!label _label)
          (Rendering|Components|TextRender|SetText (Variables|/Game/UI/UMG/UMG_Main.UMG_Main_C|GetTextBlock_提示 (Variables|/Game/ThirdPerson/Blueprints/BP_ThirdPersonCharacter.BP_ThirdPersonCharacter_C|GetUMG_Main (Variables|Default|GetAs%20BP%20Third%20Person%20Character))) "无法拾取")
          (Utilities|FlowControl|Delay 2.0)
          (Widget|SetVisibility (Variables|/Game/UI/UMG/UMG_Main.UMG_Main_C|GetTextBlock_提示 (Variables|/Game/ThirdPerson/Blueprints/BP_ThirdPersonCharacter.BP_ThirdPersonCharacter_C|GetUMG_Main (Variables|Default|GetAs%20BP%20Third%20Person%20Character))) "Hidden"))))
    (:CastFailed
      (goto _label))))

(event EventBeginPlay
  (|CallParentFunction) ; 此节点被禁用，将不会被调用。\n从引脚连出引线来编译功能。
)

(event Collision|EventActorBeginOverlap
  (params (OtherActor :type Actor%20Object%20Reference))
  (|CallParentFunction OtherActor) ; 此节点被禁用，将不会被调用。\n从引脚连出引线来编译功能。
)

(event EventTick
  (params (DeltaSeconds :type Float%20%28single-precision%29))
  (|CallParentFunction DeltaSeconds) ; 此节点被禁用，将不会被调用。\n从引脚连出引线来编译功能。
)

(fn ConstructionScript
  (|CallParentFunction))