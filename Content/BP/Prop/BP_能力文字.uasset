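; BP_能力文字 is a spinning ability-text prop that takes on a random E_Text ability when play begins.
; A Select on that ability sets the static mesh to the matching character (大, 重 or 快: big, heavy or fast).
; Tick yaws the mesh at a constant, frame-rate-independent speed.
; The Sphere overlap event is empty, so this Blueprint implements no pickup or ability effect.
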(event OnComponentBeginOverlap(Sphere)
  (params (OverlappedComponent :type Primitive%20Component%20Object%20Reference) (OtherActor :type Actor%20Object%20Reference) (OtherComp :type Primitive%20Component%20Object%20Reference) (OtherBodyIndex :type Integer) (bFromSweep :type Boolean) (SweepResult :type Hit%20Result%20Structure%20%28by%20ref%29)))

(event EventBeginPlay
  (bind _output_get (Variables|Default|Set能力 (Utilities|Enum|ByteToEnumE_Text (Math|Conversions|ToByte(Integer) (Math|Random|RandomIntegerinRange 0 3)))))
  (Components|StaticMesh|SetStaticMesh (Variables|Default|GetStaticMesh) (Utilities|Select :Index _output_get :NewEnumerator0 "/Game/BP/Prop/大.大" :NewEnumerator1 "/Game/BP/Prop/重.重" :NewEnumerator2 "/Game/BP/Prop/快.快")))

(event EventTick
  (params (DeltaSeconds :type Float%20%28single-precision%29))
  (Transformation|AddWorldRotation (Variables|Default|GetStaticMesh) (Math|Rotator|MakeRotator 0.0 0.0 (* DeltaSeconds 1e+02)) false false))

(fn ConstructionScript
  (|CallParentFunction))