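; BP_Noun is an actor Blueprint that hands out gameplay abilities to noun actors when its StartBindGA event fires.
; BeginPlay binds that event, whose handler reads parallel SN and SG arrays from BP_GameInstance.
; For each SN entry, it finds all actors of that class and gives them the matching SG ability at level 1.
; BP_NWeapon entries take a separate cast branch with the same grant logic.
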(event Custom|StartBindGA_Event
  (bind _asbp_game_instance (Utilities|Casting|CastToBP_GameInstance (Game|GetGameInstance))
    (:then
      (for (_array_element _array_index) (Variables|/Game/BP/BP_GameInstance.BP_GameInstance_C|GetSN _asbp_game_instance)
        (bind _asbp_nweapon (Utilities|Casting|CastToBP_NWeaponClass _array_element)
          (:then
            (bind _outactors (Actor|GetAllActorsOfClass _asbp_nweapon))
            (for _array_element_2 _outactors
              (bind _asbp_noun (Utilities|Casting|CastToBP_Noun _array_element_2))
              (Class|Noun|GiveAbility _asbp_noun (Utilities|Array|Get(acopy) (Variables|/Game/BP/BP_GameInstance.BP_GameInstance_C|GetSG _asbp_game_instance) _array_index) 1)))
          (:CastFailed
            (bind _outactors_2 (Actor|GetAllActorsOfClass (Utilities|Array|Get(acopy) (Variables|/Game/BP/BP_GameInstance.BP_GameInstance_C|GetSN _asbp_game_instance) _array_index)))
            (for _array_element_3 _outactors_2
              (bind _asbp_noun_2 (Utilities|Casting|CastToBP_Noun _array_element_3))
              (Class|Noun|GiveAbility _asbp_noun_2 (Utilities|Array|Get(acopy) (Variables|/Game/BP/BP_GameInstance.BP_GameInstance_C|GetSG _asbp_game_instance) _array_index) 1))))))
    (:CastFailed
      (Development|PrintString "fail"))))

(event EventBeginPlay
  (EventDispatchers|BindEventtoStartBindGA (delegate Custom|StartBindGA_Event)))

(event Collision|EventActorBeginOverlap
  (params (OtherActor :type Actor%20Object%20Reference)))

(event EventTick
  (params (DeltaSeconds :type Float%20%28single-precision%29)))

(fn ConstructionScript)