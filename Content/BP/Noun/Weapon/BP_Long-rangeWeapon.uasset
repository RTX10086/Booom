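; Ranged weapon actor that the third-person character picks up on overlapping its Cube, passing itself through BPI_PicUp for the long-weapon hand socket.
; WeaponAttackEvent plays a firing montage and immediately spawns a scaled BP_Bullte, launched by impulse along the character's MouseD direction.
; A shot counter triggers a reload montage after 30 shots and resets when it completes.
; The IsShooting flag clears right after spawning, without waiting for the montage.
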(event OnComponentBeginOverlap(Cube)
  (params (OverlappedComponent :type Primitive%20Component%20Object%20Reference) (OtherActor :type Actor%20Object%20Reference) (OtherComp :type Primitive%20Component%20Object%20Reference) (OtherBodyIndex :type Integer) (bFromSweep :type Boolean) (SweepResult :type Hit%20Result%20Structure%20%28by%20ref%29))
  (bind _asbp_third_person_character (Utilities|Casting|CastToBP_ThirdPersonCharacter OtherActor))
  (bind _output_get (Variables|Default|SetAs%20BP%20Third%20Person%20Character _asbp_third_person_character))
  (bind _asbpi_pic_up (Utilities|Casting|CastToBPI_PicUp _output_get))
  (Default|PickUp _asbpi_pic_up self "Hand_r_Weapon_Long"))

(event EventBeginPlay
  (|CallParentFunction) ; 此节点被禁用，将不会被调用。\n从引脚连出引线来编译功能。
)

(event Collision|EventActorBeginOverlap
  (params (OtherActor :type Actor%20Object%20Reference))
  (|CallParentFunction OtherActor) ; 此节点被禁用，将不会被调用。\n从引脚连出引线来编译功能。
)

(event EventTick
  (params (DeltaSeconds :type Float%20%28single-precision%29))
  (|CallParentFunction DeltaSeconds) ; 此节点被禁用，将不会被调用。\n从引脚连出引线来编译功能。
)

(event EventWeaponAttackEvent
  (bind _spawn_transform_scale (Variables|Default|GetSpawn%20Transform%20Scale))
  (bind _cube (Variables|Default|GetCube))
  (bind _as_bp_third_person_character (Variables|Default|GetAs%20BP%20Third%20Person%20Character))
  (bind _bulletsize (Variables|Default|GetBulletSize))
  (bind _returnvalue (Transformation|GetWorldTransform _cube))
  (bind _mesh (Variables|/Script/Engine.Character|GetMesh _as_bp_third_person_character))
  (bind _moused (Variables|/Game/ThirdPerson/Blueprints/BP_ThirdPersonCharacter.BP_ThirdPersonCharacter_C|GetMouseD _as_bp_third_person_character))
  (if (<= (Variables|Default|GetNewVar_0) 29)
    (if (not (Variables|Default|GetIsShooting))
      (Variables|Default|SetIsShooting true)
      (Animation|Montage|PlayMontage _mesh "/Game/Characters/Mannequin_UE4/Test/Anim_BP/Firing_Rifle__2__Montage.Firing_Rifle__2__Montage" 0.5
        (:then
          (bind _returnvalue_2 (Game|SpawnActorfromClass "/Game/BP/Noun/Weapon/BP_Bullte.BP_Bullte_C" (Math|Transform|MakeTransform (+ (.location _returnvalue) (* _moused 25.0)) (.rotation _returnvalue) (Math|Vector|MakeVector (.x _spawn_transform_scale) (+ (.y _spawn_transform_scale) _bulletsize) (+ (.z _spawn_transform_scale) _bulletsize))) "Undefined" 0 0))
          (Physics|AddImpulse (Variables|/Game/BP/Noun/Weapon/BP_Bullte.BP_Bullte_C|GetStaticMesh _returnvalue_2) (* _moused 2.5e+03) "None" false)
          (Variables|Default|SetNewVar_0 (+ (Variables|Default|GetNewVar_0) 1))
          (Variables|Default|SetIsShooting false))))
    (elif (not (Variables|Default|GetIsReloding))
      (Variables|Default|SetIsReloding true)
      (Animation|Montage|PlayMontage _mesh "/Game/Characters/Mannequin_UE4/Test/Anim_BP/Reload_Montage.Reload_Montage"
        (:OnCompleted
          (Variables|Default|SetNewVar_0 0)
          (Variables|Default|SetIsReloding false))))))

(fn ConstructionScript
  (|CallParentFunction))