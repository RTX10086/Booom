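; Baseball bat weapon actor that can be picked up and triggers an attack when it touches an enemy.
; Overlap on its Cube passes the bat to any BPI_PicUp implementer for the right-hand weapon socket.
; The same overlap stores a BP_NEnemy as Target and activates GA_Attack through the Ability System Component.
; AttackFlag and a two-second Delay act as a cooldown between attacks.
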(event OnComponentBeginOverlap(Cube)
  (params (OverlappedComponent :type Primitive%20Component%20Object%20Reference) (OtherActor :type Actor%20Object%20Reference) (OtherComp :type Primitive%20Component%20Object%20Reference) (OtherBodyIndex :type Integer) (bFromSweep :type Boolean) (SweepResult :type Hit%20Result%20Structure%20%28by%20ref%29))
  (Utilities|FlowControl|Sequence
    (:then_0
      (bind _asbpi_pic_up (Utilities|Casting|CastToBPI_PicUp OtherActor))
      (Default|PickUp _asbpi_pic_up self "Hand_r_Weapon"))
    (:then_1
      (bind _asbp_nenemy (Utilities|Casting|CastToBP_NEnemy OtherActor))
      (if (Variables|Default|GetAttackFlag)
        (Variables|Default|SetAttackFlag false)
        (Variables|Default|SetTarget _asbp_nenemy)
        (Abilities|TryActivateAbilitybyClass (Variables|Default|GetAbilitySystemComponent) "/Game/GAS/GA/GA_Attack.GA_Attack_C" true)
        (Utilities|FlowControl|Delay 2.0)
        (Variables|Default|SetAttackFlag true)))))

(event EventBeginPlay
  (|CallParentFunction) ; 此节点被禁用，将不会被调用。\n从引脚连出引线来编译功能。
)

(event Collision|EventActorBeginOverlap
  (params (OtherActor :type Actor%20Object%20Reference))
  (|CallParentFunction OtherActor) ; 此节点被禁用，将不会被调用。\n从引脚连出引线来编译功能。
)

(event EventTick
  (params (DeltaSeconds :type Float%20%28single-precision%29))
  (|CallParentFunction DeltaSeconds) ; 此节点被禁用，将不会被调用。\n从引脚连出引线来编译功能。
)

(fn ConstructionScript
  (|CallParentFunction))