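; Robot enemy that chases and punches the player, using Gameplay Ability System abilities for attacks and stat setup.
; Pawn sensing starts AIMoveTo, Tick adds forward force during the chase, and arrival triggers the punch montage with GA_Attack.
; Capsule overlaps store knockback from bullets or weapons.
; When its attribute depletes, it plays death, spawns GAObject or MedicalKit (SpeedUP case is unreachable), and destroys itself on the "Dead" notify.
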(event OnComponentBeginOverlap(CapsuleComponent)
  (params (OverlappedComponent :type Primitive%20Component%20Object%20Reference) (OtherActor :type Actor%20Object%20Reference) (OtherComp :type Primitive%20Component%20Object%20Reference) (OtherBodyIndex :type Integer) (bFromSweep :type Boolean) (SweepResult :type Hit%20Result%20Structure%20%28by%20ref%29))
  (|CallParentFunction)
  (bind _knockback (CallFunction|SetKnockback OtherActor))
  (Variables|Default|SetKnockback _knockback))

(event OnSeePawn(AiMove)
  (params (Pawn :type Pawn%20Object%20Reference))
  (bind _asbp_third_person_character (Utilities|Casting|CastToBP_ThirdPersonCharacter Pawn))
  (AI|AIMoveTo self "0, 0, 0" _asbp_third_person_character 5.0 false
    (:then
      (Variables|Default|SetNewVar true))
    (:OnSuccess
      (Variables|Default|SetNewVar false)
      (Animation|Montage|PlayMontage (Variables|Character|GetMesh) "/Game/BP/Noun/Enemy/Robot/Animation/Robot_Punch_AnimMontage.Robot_Punch_AnimMontage" (Variables|Default|GetPlay%20Rate)
        (:then
          (Abilities|TryActivateAbilitybyClass (Variables|Default|GetAbilitySystemComponent) "/Game/GAS/GA/GA_Attack.GA_Attack_C" true))))))

(event EventBeginPlay
  (|CallParentFunction)
  (bind _knockback (CallFunction|SetKnockback (stale OnComponentBeginOverlap(CapsuleComponent) OtherActor)))
  (Variables|Default|SetKnockback _knockback))

(event Collision|EventActorBeginOverlap
  (params (OtherActor :type Actor%20Object%20Reference))
  (|CallParentFunction OtherActor) ; 此节点被禁用，将不会被调用。\n从引脚连出引线来编译功能。
)

(event EventTick
  (params (DeltaSeconds :type Float%20%28single-precision%29))
  (bind _capsulecomponent (Variables|Default|GetCapsuleComponent))
  (bind _returnvalue (Transformation|GetWorldTransform _capsulecomponent))
  (if (> (.ReturnValue (Ability|Attribute|GetFloatAttribute self "(AttributeName=\"Health\",Attribute=/Script/Booom.CharactorAttributeSet:Health,AttributeOwner=/Script/CoreUObject.Class'\"/Script/Booom.CharactorAttributeSet\"')")) 0.0)
    (if (Variables|Default|GetNewVar)
      (Physics|AddForce (Variables|Default|GetCapsuleComponent) (* (Math|Vector|GetForwardVector (Variables|Default|GetCapsuleComponent)) (Variables|Default|GetEnemySpeed)) "None" false))
    (else
      (Utilities|FlowControl|DoOnce false
        (:Completed
          (Utilities|FlowControl|Sequence
            (:then_0
              (bind _notifyname (Animation|Montage|PlayMontage (Variables|Character|GetMesh) "/Game/BP/Noun/Enemy/Robot/Animation/Robot_Death_AnimMontage.Robot_Death_AnimMontage")
                (:then
                  (Variables|Default|SetIsDeath true))
                (:OnNotifyBegin
                  (if (== _notifyname "Dead")
                    (Actor|DestroyActor)))))
            (:then_1
              (switch int (Math|Random|RandomInteger 2)
                (:0
                  (Variables|Default|SetClass "/Game/BP/NPC/GAObject.GAObject_C"))
                (:1
                  (Variables|Default|SetClass "/Game/BP/NPC/MedicalKit.MedicalKit_C"))
                (:2
                  (Variables|Default|SetClass "/Game/BP/NPC/SpeedUP.SpeedUP_C")))
              (Audio|PlaySound2D "/Engine/VREditor/Sounds/VR_click1_Cue.VR_click1_Cue" 1.0 1.0 0.0 0 0)
              (Game|SpawnActorfromClass (Variables|Default|GetClass) (Math|Transform|MakeTransform (.location _returnvalue) (.rotation _returnvalue) "0.100000,0.100000,0.100000") "Undefined" 0 0))))))))

(event EventTryGA
  (params (NewParam :type Integer))
  (bind _returnvalue (Abilities|TryActivateAbilitybyClass (Variables|Default|GetAbilitySystemComponent) "/Game/GAS/GA/GA_SetSize.GA_SetSize_C" true))
  (Abilities|TryActivateAbilitybyClass (Variables|Default|GetAbilitySystemComponent) "/Game/GAS/GA/GA_SetSpeed1.GA_SetSpeed1_C" true)
  (Abilities|TryActivateAbilitybyClass (Variables|Default|GetAbilitySystemComponent) "/Game/GAS/GA/GA_SetPlayRate.GA_SetPlayRate_C" true)
  (Development|PrintString (Utilities|String|ToString(Boolean) _returnvalue)))

(fn ConstructionScript
  (|CallParentFunction))

(fn SetKnockback
  (params (Item :type Actor%20Object%20Reference))
  (bind _asbp_bullte (Utilities|Casting|CastToBP_Bullte Item)
    (:then
      (LocalVariables|SetReturn (Variables|/Game/BP/Noun/Weapon/BP_Bullte.BP_Bullte_C|GetKnockback _asbp_bullte)))
    (:CastFailed
      (bind _asbp_nweapon (Utilities|Casting|CastToBP_NWeapon Item))
      (LocalVariables|SetReturn (Variables|/Game/BP/Noun/Weapon/BP_NWeapon.BP_NWeapon_C|GetKnockback _asbp_nweapon))))
  (return (LocalVariables|GetReturn)))