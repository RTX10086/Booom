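; Enemy character that chases a seen player, shoots when within 1000 units, and drops a pickup on death.
; Pawn sensing starts AI movement and the rifle montage with an impulse-launched bullet; Tick adds forward force when distant.
; A depleted GAS attribute triggers the death montage and random drop, though RandomInteger(2) never selects SpeedUP.
; TryGA activates size, speed and play-rate abilities.
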(event OnSeePawn(AiMove)
  (params (Pawn :type Pawn%20Object%20Reference))
  (bind _self self)
  (bind _returnvalue (Transformation|GetActorTransform _self))
  (Utilities|Casting|CastToBP_ThirdPersonCharacter Pawn)
  (AI|AIMoveTo self "0, 0, 0" 0 5.0 false
    (:then
      (Variables|Default|SetNewVar true)
      (if (not (stale EventTick _output_get))
        (Utilities|FlowControl|Delay (/ 0.4 (Variables|Default|GetPlay%20Rate)))
        (Utilities|FlowControl|DoOnce false :!label _label
          (:Completed
            (Animation|Montage|PlayMontage (Variables|Character|GetMesh) "/Game/BP/Noun/Enemy/Enemy_Long/Firing_Rifle__2_2_Montage.Firing_Rifle__2_2_Montage" 0.8
              (:then
                (bind _returnvalue_2 (Game|SpawnActorfromClass "/Game/BP/Noun/Weapon/BP_Bullte1.BP_Bullte1_C" (Math|Transform|MakeTransform (.location _returnvalue) (.rotation _returnvalue) "0.500000,0.100000,0.100000") "Undefined" 0 0))
                (Physics|AddImpulse (Variables|/Game/BP/Noun/Weapon/BP_Bullte1.BP_Bullte1_C|GetStaticMesh _returnvalue_2) (* (Math|Vector|GetForwardVector (Variables|/Game/BP/Noun/Weapon/BP_Bullte1.BP_Bullte1_C|GetStaticMesh _returnvalue_2)) 5e+02) "None" false)
                (Variables|Default|SetNewVar false)
                (goto _label Reset)))))))))

(event EventBeginPlay)

(event Collision|EventActorBeginOverlap
  (params (OtherActor :type Actor%20Object%20Reference)))

(event EventTryGA
  (params (NewParam :type Integer))
  (Abilities|TryActivateAbilitybyClass (Variables|Default|GetAbilitySystemComponent) "/Game/GAS/GA/GA_SetSize.GA_SetSize_C" true)
  (Abilities|TryActivateAbilitybyClass (Variables|Default|GetAbilitySystemComponent) "/Game/GAS/GA/GA_SetSpeed1.GA_SetSpeed1_C" true)
  (Abilities|TryActivateAbilitybyClass (Variables|Default|GetAbilitySystemComponent) "/Game/GAS/GA/GA_SetPlayRate.GA_SetPlayRate_C" true)
  (Development|PrintString "Hello"))

(event EventTick
  (params (DeltaSeconds :type Float%20%28single-precision%29))
  (bind _capsulecomponent (Variables|Default|GetCapsuleComponent))
  (bind _returnvalue (Transformation|GetWorldTransform _capsulecomponent))
  (if (> (.ReturnValue (Ability|Attribute|GetFloatAttribute self "(AttributeName=\"Health\",Attribute=/Script/Booom.CharactorAttributeSet:Health,AttributeOwner=/Script/CoreUObject.Class'\"/Script/Booom.CharactorAttributeSet\"')")) 0.0)
    (Utilities|FlowControl|Sequence
      (:then_0
        (if (stale _output_get)
          (if (Variables|Default|GetNewVar)
            (Physics|AddForce (Variables|Default|GetCapsuleComponent) (* (Math|Vector|GetForwardVector (Variables|Default|GetCapsuleComponent)) (Variables|Default|GetEnemySpeed)) "None" false))))
      (:then_1
        (bind _returnvalue_2 (Actor|GetActorOfClass "/Game/ThirdPerson/Blueprints/BP_ThirdPersonCharacter.BP_ThirdPersonCharacter_C"))
        (bind _output_get (Variables|Default|SetIsAttack (> (Math|Vector|VectorLength (- (Transformation|GetWorldLocation (Variables|/Script/Engine.Actor|GetRootComponent _returnvalue_2)) (Transformation|GetWorldLocation (Variables|Default|GetCapsuleComponent)))) 1e+03)))))
    (else
      (Utilities|FlowControl|DoOnce false
        (:Completed
          (Utilities|FlowControl|Sequence
            (:then_0
              (Variables|Default|SetIsDeath true)
              (bind _notifyname (Animation|Montage|PlayMontage (Variables|Character|GetMesh) "/Game/BP/Noun/Enemy/Enemy_Long/Dying_Montage.Dying_Montage" 3.0)
                (:OnInterrupted
                  (Actor|DestroyActor :!label _label))
                (:OnNotifyBegin
                  (if (== _notifyname "Dead")
                    (goto _label)))))
            (:then_1
              (switch int (Math|Random|RandomInteger 2)
                (:0
                  (Variables|Default|SetClass_0 "/Game/BP/NPC/GAObject.GAObject_C"))
                (:1
                  (Variables|Default|SetClass_0 "/Game/BP/NPC/MedicalKit.MedicalKit_C"))
                (:2
                  (Variables|Default|SetClass_0 "/Game/BP/NPC/SpeedUP.SpeedUP_C")))
              (Audio|PlaySound2D "/Engine/VREditor/Sounds/VR_click1_Cue.VR_click1_Cue" 1.0 1.0 0.0 0 0)
              (Game|SpawnActorfromClass (Variables|Default|GetClass_0) (Math|Transform|MakeTransform (.location _returnvalue) (.rotation _returnvalue) "0.100000,0.100000,0.100000") "Undefined" 0 0))))))))

(fn ConstructionScript
  (|CallParentFunction))