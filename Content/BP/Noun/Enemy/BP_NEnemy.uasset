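; BP_NEnemy is an enemy actor that uses the Gameplay Ability System and reacts to overlaps on its Cube.
; An overlap stores bullet or weapon knockback, picks a random GALib item, and triggers GA_Attack on an overlapping third-person character.
; BeginPlay shares that same overlap chain.
; Tick uses a three-second Delay to repeatedly activate GA_FireDamage on itself and print an attribute value.
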(event OnComponentBeginOverlap(Cube)
  (params (OverlappedComponent :type Primitive%20Component%20Object%20Reference) (OtherActor :type Actor%20Object%20Reference) (OtherComp :type Primitive%20Component%20Object%20Reference) (OtherBodyIndex :type Integer) (bFromSweep :type Boolean) (SweepResult :type Hit%20Result%20Structure%20%28by%20ref%29))
  (|CallParentFunction)
  (bind _knockback (CallFunction|SetKnockback OtherActor))
  (Variables|Default|SetKnockback _knockback)
  (bind _asbp_game_instance (Utilities|Casting|CastToBP_GameInstance (Game|GetGameInstance)))
  (Variables|Default|SetAddGAItem (.OutItem (Utilities|Array|Random (Variables|/Game/BP/BP_GameInstance.BP_GameInstance_C|GetGALib _asbp_game_instance))))
  (bind _asbp_third_person_character (Utilities|Casting|CastToBP_ThirdPersonCharacter OtherActor))
  (Abilities|TryActivateAbilitybyClass (Variables|/Script/Booom.BooomCharacter|GetAbilitySystemComponent _asbp_third_person_character) "/Game/GAS/GA/GA_Attack.GA_Attack_C" true))

(event EventBeginPlay
  (|CallParentFunction)
  (bind _knockback (CallFunction|SetKnockback (stale OnComponentBeginOverlap(Cube) OtherActor)))
  (Variables|Default|SetKnockback _knockback)
  (bind _asbp_game_instance (Utilities|Casting|CastToBP_GameInstance (Game|GetGameInstance)))
  (Variables|Default|SetAddGAItem (.OutItem (Utilities|Array|Random (Variables|/Game/BP/BP_GameInstance.BP_GameInstance_C|GetGALib _asbp_game_instance))))
  (bind _asbp_third_person_character (Utilities|Casting|CastToBP_ThirdPersonCharacter (stale OnComponentBeginOverlap(Cube) OtherActor)))
  (Abilities|TryActivateAbilitybyClass (Variables|/Script/Booom.BooomCharacter|GetAbilitySystemComponent _asbp_third_person_character) "/Game/GAS/GA/GA_Attack.GA_Attack_C" true))

(event Collision|EventActorBeginOverlap
  (params (OtherActor :type Actor%20Object%20Reference))
  (|CallParentFunction OtherActor) ; 此节点被禁用，将不会被调用。\n从引脚连出引线来编译功能。
)

(event EventTick
  (params (DeltaSeconds :type Float%20%28single-precision%29))
  (|CallParentFunction DeltaSeconds)
  (Utilities|FlowControl|Delay 3.0)
  (Utilities|FlowControl|Sequence
    (:then_0
      (Abilities|TryActivateAbilitybyClass (Variables|Default|GetAbilitySystemComponent) "/Game/GAS/GA/GA_FireDamage.GA_FireDamage_C" true))
    (:then_1
      (Development|PrintString (Utilities|String|ToString(Float) (.ReturnValue (Ability|Attribute|GetFloatAttribute self "(AttributeName=\"Health\",Attribute=/Script/Booom.CharactorAttributeSet:Health,AttributeOwner=/Script/CoreUObject.Class'\"/Script/Booom.CharactorAttributeSet\"')")))))))

(fn ConstructionScript
  (|CallParentFunction))

(fn SetKnockback
  (params (Item :type Actor%20Object%20Reference))
  (bind _asbp_bullte (Utilities|Casting|CastToBP_Bullte Item)
    (:then
      (LocalVariables|SetReturn (Variables|/Game/BP/Noun/Weapon/BP_Bullte.BP_Bullte_C|GetKnockback _asbp_bullte)))
    (:CastFailed
      (bind _asbp_nweapon (Utilities|Casting|CastToBP_NWeapon Item))
      (LocalVariables|SetReturn (Variables|/Game/BP/Noun/Weapon/BP_NWeapon.BP_NWeapon_C|GetKnockback _asbp_nweapon))))
  (return (LocalVariables|GetReturn)))